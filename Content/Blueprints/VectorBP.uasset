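; VectorBP is an actor that wanders endlessly between random points at a fixed height, moved by manual vector math.
; SetRandomDestination picks a point in a square around the world origin at BeginPlay and again on each arrival.
; Tick normalizes the offset to that point and moves by direction, Speed and DeltaSeconds without sweeping.
; Arrival means the distance drops below Speed, roughly one second of travel.
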(event `self.ReceiveBeginPlay`
  (`self.SetRandomDestination`))

(event `self.ReceiveTick`
  (params (DeltaSeconds :type "Float (single-precision)"))
  (set `self.DeltaSeconds` DeltaSeconds)
  (set `self.vDistance` (- (`self.vDestination`) (`self.K2_GetActorLocation`)))
  (set `self.vDirection` (`KismetMathLibrary.Normal` (`self.vDistance`) 0.0))
  (set `self.vVelocity` (* (`self.vDirection`) (`self.Speed`)))
  (set `self.vStep` (* (`self.vVelocity`) (`self.DeltaSeconds`)))
  (`self.K2_AddActorWorldOffset` (`self.vStep`))
  (if (< (`KismetMathLibrary.VSize` (`self.vDistance`)) (`self.Speed`))
    (`self.SetRandomDestination`)))

(fn `UserConstructionScript`)